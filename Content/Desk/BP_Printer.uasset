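; BP_Printer is an interactable desk printer that starts the game for the interacting character.
; While the game has not started, the trace event shows or hides its TextRender based on whether the printer is interactable.
; Interaction hides the text, sets the character's Started flag and calls StartGame, so both events do nothing afterward for that character.
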(event `/Game/InteractableSystem/BPI_Interactable.Interaction`
  (params (InteractingCharacter :type "/Game/FirstPerson/Blueprints/BP_FirstPersonCharacter Object Reference"))
  (if (not (`/Game/FirstPerson/Blueprints/BP_FirstPersonCharacter.Started` InteractingCharacter))
    (`SceneComponent.SetVisibility` (`self.TextRender`) false false)
    (set `/Game/FirstPerson/Blueprints/BP_FirstPersonCharacter.Started` true InteractingCharacter)
    (`/Game/FirstPerson/Blueprints/BP_FirstPersonCharacter.StartGame` InteractingCharacter)))

(event `/Game/InteractableSystem/BPI_Interactable.CanRecieveTrace`
  (params (Interactable :type Boolean) (InteractingCharacter :type "/Game/FirstPerson/Blueprints/BP_FirstPersonCharacter Object Reference"))
  (bind _textrender (`self.TextRender`))
  (if (`/Game/FirstPerson/Blueprints/BP_FirstPersonCharacter.Started` InteractingCharacter)
    _
    (elif Interactable
      (`SceneComponent.SetVisibility` _textrender true false)
      (else
        (`SceneComponent.SetVisibility` _textrender false false)))))

(fn `UserConstructionScript`)