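; BP_SpareButton is a desk button that reacts visually when the first-person character signals an approval.
; On BeginPlay it sets a basic material and binds its Approve event to the player character's approve dispatcher.
; Approve turns the button emissive green and plays a timeline that lerps it downward, restoring the basic material on finish.
; The timeline uses Play rather than PlayFromStart, and nothing moves the button back up.
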(event `self.ReceiveBeginPlay`
  (`PrimitiveComponent.SetMaterial` (`self.Button`) 0 "/Game/StarterContent/Materials/M_Basic_Floor.M_Basic_Floor")
  (bind _asbp_first_person_character (cast `/Game/FirstPerson/Blueprints/BP_FirstPersonCharacter` (`GameplayStatics.GetPlayerCharacter` 0)))
  (add `/Game/FirstPerson/Blueprints/BP_FirstPersonCharacter.ApproveDispatcher` _asbp_first_person_character (delegate `approve`)))

(event `approve`
  (bind _button (`self.Button`))
  (`PrimitiveComponent.SetMaterial` _button 0 "/Engine/ArtTools/RenderToTexture/Materials/Debug/M_Emissive_green.M_Emissive_green")
  (bind (_direction _buttonpress _lerpalha) (`Timeline|ButtonTimeline`)
    (:`Update`
      (`SceneComponent.K2_SetRelativeLocation` (`self.Button`) (`KismetMathLibrary.VLerp` (0.0 0.0 33.0) (0.0 0.0 13.916184) _lerpalha) false false))
    (:`Finished`
      (`PrimitiveComponent.SetMaterial` _button 0 "/Game/StarterContent/Materials/M_Basic_Floor.M_Basic_Floor"))))

(fn `UserConstructionScript`)