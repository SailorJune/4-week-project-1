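; Desk button actor that lets the first-person player pass a condemn verdict when ReadyToJudge is set.
; Trace feedback toggles CondemnRender, and interacting hides it and calls Condemn on the character.
; Character dispatchers, bound at BeginPlay, drive timelines that raise the initially lowered button or sink it on condemn, with material swaps around the press.
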(event `/Game/InteractableSystem/BPI_Interactable.Interaction`
  (params (InteractingCharacter :type "/Game/FirstPerson/Blueprints/BP_FirstPersonCharacter Object Reference"))
  (if (`/Game/FirstPerson/Blueprints/BP_FirstPersonCharacter.ReadyToJudge` InteractingCharacter)
    (`SceneComponent.SetVisibility` (`self.CondemnRender`) false false)
    (`/Game/FirstPerson/Blueprints/BP_FirstPersonCharacter.Condemn` InteractingCharacter)))

(event `/Game/InteractableSystem/BPI_Interactable.CanRecieveTrace`
  (params (Interactable :type Boolean) (InteractingCharacter :type "/Game/FirstPerson/Blueprints/BP_FirstPersonCharacter Object Reference"))
  (bind _condemnrender (`self.CondemnRender`))
  (if (`/Game/FirstPerson/Blueprints/BP_FirstPersonCharacter.ReadyToJudge` InteractingCharacter)
    (if Interactable
      (`SceneComponent.SetVisibility` _condemnrender true false)
      (else
        (`SceneComponent.SetVisibility` _condemnrender false false)))))

(event `self.ReceiveBeginPlay`
  (`SceneComponent.K2_SetRelativeLocation` (`self.Button`) (0.0 0.0 13.916184) false false)
  (`PrimitiveComponent.SetMaterial` (`self.Button`) 0 "/Game/StarterContent/Materials/M_Basic_Floor.M_Basic_Floor")
  (bind _asbp_first_person_character (cast `/Game/FirstPerson/Blueprints/BP_FirstPersonCharacter` (`GameplayStatics.GetPlayerCharacter` 0)))
  (add `/Game/FirstPerson/Blueprints/BP_FirstPersonCharacter.CondomnDispatcher` _asbp_first_person_character (delegate `condemn`))
  (add `/Game/FirstPerson/Blueprints/BP_FirstPersonCharacter.ButtonRiseDispatcher` _asbp_first_person_character (delegate `Become Clickable`)))

(event `condemn`
  (bind _button (`self.Button`))
  (`PrimitiveComponent.SetMaterial` _button 0 null)
  (bind (_direction _buttonpress _newtrack_0) (`Timeline|Timeline`)
    (:`Update`
      (`SceneComponent.K2_SetRelativeLocation` _button (`KismetMathLibrary.VLerp` (0.0 0.0 33.0) (0.0 0.0 13.916184) _newtrack_0) false false))
    (:`Finished`
      (`PrimitiveComponent.SetMaterial` _button 0 "/Game/StarterContent/Materials/M_Basic_Floor.M_Basic_Floor"))))

(event `Become Clickable`
  (bind (_direction _newtrack_0) (`Timeline|TimelineRise`)
    (:`Update`
      (`SceneComponent.K2_SetRelativeLocation` (`self.Button`) (`KismetMathLibrary.VLerp` (0.0 0.0 13.916184) (0.0 0.0 33.0) _newtrack_0) false false))))

(fn `UserConstructionScript`)